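; BP_MovingPiston is an actor that moves vertically between its placed location and a point offset by OffsetHeight.
; On BeginPlay it stores its starting position, waits StartTimeOffset seconds, then plays the Movingpiston timeline.
; Each timeline update lerps the whole actor's location along Z without sweeping, and the delay lets instances start at different times.
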(event `self.ReceiveBeginPlay`
  (set `self.InitialPos` (`self.K2_GetActorLocation`))
  (`KismetSystemLibrary.Delay` (`self.StartTimeOffset`))
  (bind (_direction _newtrack_0) (`Timeline|movingpiston`)
    (:`Update`
      (`self.K2_SetActorLocation` (`KismetMathLibrary.VLerp` (`self.InitialPos`) (+ (`self.InitialPos`) (`KismetMathLibrary.MakeVector` 0.0 0.0 (`self.OffsetHeight`))) _newtrack_0)))))

(fn `UserConstructionScript`)