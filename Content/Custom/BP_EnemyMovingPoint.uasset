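; BP_EnemyMovingPoint is a waypoint that moves an enemy along a linked chain of points.
; The current point rotates its enemy toward NextPointInLine and lerps it there on Tick using real time, then hands it over on arrival.
; Travel duration is distance multiplied by MovementSpeed, so higher values move slower.
; The construction script stretches a cube toward the next point and, if that link exists, greens the sphere when an enemy is assigned.
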(event `RecieveSwitchPoint`
  (bind (_seconds _partialseconds) (`GameplayStatics.GetAccurateRealTime`))
  (set `self.InitialTime` (+ _seconds _partialseconds))
  (`self.K2_SetActorRotation` (`self.OwningEnemy`) (`KismetMathLibrary.FindLookAtRotation` (`self.K2_GetActorLocation`) (`self.K2_GetActorLocation` (`self.NextPointInLine`))) false)
  (set `self.EnemyMovementSpeed` (`/Game/Custom/BP_Enemy.MovementSpeed` (`self.OwningEnemy`))))

(event `self.ReceiveBeginPlay`
  (`/Engine/EditorBlueprintResources/StandardMacros.IsValid` (`self.OwningEnemy`)
    (:`Is Valid`
      (set `self.IsCurrentPoint` true)
      (`self.RecieveSwitchPoint`))))

(event `self.ReceiveTick`
  (params (DeltaSeconds :type "Float (single-precision)"))
  (bind (_seconds _partialseconds) (`GameplayStatics.GetAccurateRealTime`))
  (bind _initialtime (`self.InitialTime`))
  (bind _nextpointinline (`self.NextPointInLine`))
  (if (`self.IsCurrentPoint`)
    (set `self.RealTime` (+ _seconds _partialseconds))
    (bind _output_get (set `self.LerpValue` (`KismetMathLibrary.MapRangeClamped` (`self.RealTime`) _initialtime (+ _initialtime (* (`KismetMathLibrary.Vector_Distance` (`self.K2_GetActorLocation`) (`self.K2_GetActorLocation` (`self.NextPointInLine`))) (`self.EnemyMovementSpeed`))) 0.0 1.0)))
    (`self.K2_SetActorLocation` (`self.OwningEnemy`) (`KismetMathLibrary.VLerp` (`self.K2_GetActorLocation`) (`self.K2_GetActorLocation` (`self.NextPointInLine`)) _output_get) false false)
    (if (>= (`self.LerpValue`) 1.0)
      (set `/Game/Custom/BP_EnemyMovingPoint.OwningEnemy` (`self.OwningEnemy`) _nextpointinline)
      (set `/Game/Custom/BP_EnemyMovingPoint.IsCurrentPoint` true _nextpointinline)
      (`self.RecieveSwitchPoint` _nextpointinline)
      (set `self.IsCurrentPoint` false))))

(fn `UserConstructionScript`
  (bind _returnvalue (`self.K2_GetActorLocation`))
  (bind _nextpointinline (`self.NextPointInLine`))
  (bind _offsetorigincube (`self.OffsetOriginCube`))
  (bind _returnvalue_2 (`self.K2_GetActorLocation` _nextpointinline))
  (`/Engine/EditorBlueprintResources/StandardMacros.IsValid` _nextpointinline
    (:`Is Valid`
      (`SceneComponent.K2_SetWorldRotation` _offsetorigincube (`KismetMathLibrary.FindLookAtRotation` _returnvalue _returnvalue_2) false false)
      (`SceneComponent.SetWorldScale3D` _offsetorigincube (`KismetMathLibrary.MakeVector` (/ (`KismetMathLibrary.Vector_Distance` _returnvalue _returnvalue_2) 200.0) 0.03 0.03))
      (`/Engine/EditorBlueprintResources/StandardMacros.IsValid` (`self.OwningEnemy`)
        (:`Is Valid`
          (`PrimitiveComponent.SetMaterial` (`self.Sphere`) 0 "/AnimationSharing/AnimSharingGreen.AnimSharingGreen"))))))